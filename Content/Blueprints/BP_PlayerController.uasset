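; BP_PlayerController is a player controller with debug-style key bindings for hosting and joining test multiplayer sessions.
; H creates "TestSession" on ThirdPersonMap through the TestGameInstance, fetched by a cast helper.
; C starts a session search on that instance, waits a fixed delay rather than a completion callback, then joins the first result or prints that none exist.
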(event `self.ReceiveBeginPlay`)

(event `Key|H`
  (params (Key :type "Key Structure"))
  (:`Pressed`
    (`TestGameInstance.createSession` (`self.GetGameInstance`) "TestSession" "/Game/ThirdPerson/Maps/ThirdPersonMap.ThirdPersonMap")))

(event `Key|C`
  (params (Key :type "Key Structure"))
  (bind _sessions_data (`self.Sessions Data`))
  (:`Pressed`
    (`TestGameInstance.findSessions` (`self.GetGameInstance`) (`self.Sessions Data`))
    (`KismetSystemLibrary.Delay` 10.0)
    (if (`KismetArrayLibrary.Array_IsNotEmpty` _sessions_data)
      (`JoinSessionCallbackProxy.JoinSession` self (`|GetArrayItem` _sessions_data))
      (else
        (`KismetSystemLibrary.PrintString` "No sessions" true true (struct :`G` 0.66 :`B` 1.0 :`A` 1.0) 10.0)))))

(fn `GetGameInstance`
  (returns (`AsTest Game Instance` :type "TestGameInstance Object Reference"))
  (bind _astest_game_instance (cast `TestGameInstance` (`GameplayStatics.GetGameInstance`)))
  (return _astest_game_instance))

(fn `UserConstructionScript`)